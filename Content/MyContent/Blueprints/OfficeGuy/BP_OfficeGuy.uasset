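; BP_OfficeGuy is the player-controlled office worker character, which can carry and use up one object at a time.
; Axis inputs move it along fixed world axes, and BeginPlay activates its Camera1 component.
; PickupObject spawns the given class attached at the HeldObject socket, while UseObject clears and destroys it.
; Pressing Use empty-handed plays a use animation, briefly disabling movement before restoring walking and the animation Blueprint.
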(event `UseObject`
  (set `self.HeldObject` null)
  (`self.K2_DestroyActor` (`self.HeldObjectInstance`)))

(event `PickupObject`
  (params (PickedUpObject :type "Actor Class Reference"))
  (set `self.HeldObject` PickedUpObject)
  (bind _returnvalue (`|SpawnActorFromClass` (`self.HeldObject`) (`KismetMathLibrary.MakeTransform` (50.0 0.0 0.0) (struct :`Yaw` 90.0)) "Undefined" "OverrideRootScale" self null))
  (set `self.HeldObjectInstance` _returnvalue)
  (`self.K2_AttachToActor` _returnvalue self "HeldObject" "KeepRelative" "KeepRelative" "KeepRelative" true))

(event `InputAxis|MoveForward`
  (params (AxisValue :type "Float (single-precision)"))
  (`PawnMovementComponent.AddInputVector` (`self.CharacterMovement`) (* (1.0 0.0 0.0) AxisValue) false))

(event `InputAxis|MoveRight`
  (params (AxisValue :type "Float (single-precision)"))
  (`PawnMovementComponent.AddInputVector` (`self.CharacterMovement`) (* (0.0 1.0 0.0) AxisValue) false))

(event `InputAction|Use`
  (params (Key :type "Key Structure"))
  (:`Pressed`
    (if (== (`self.HeldObject`) null)
      (`SkeletalMeshComponent.PlayAnimation` (`self.Mesh`) "/Game/MyContent/Blueprints/OfficeGuy/GDTB_OfficeGuy_Anim_OfficeGuy_Use.GDTB_OfficeGuy_Anim_OfficeGuy_Use" false)
      (`CharacterMovementComponent.SetMovementMode` (`self.CharacterMovement`) "MOVE_None" 0)
      (`KismetSystemLibrary.Delay` 0.25)
      (`CharacterMovementComponent.SetMovementMode` (`self.CharacterMovement`) "MOVE_Walking" 0)
      (`SkeletalMeshComponent.SetAnimationMode` (`self.Mesh`) "AnimationBlueprint"))))

(event `self.ReceiveBeginPlay`
  (`ActorComponent.Activate` (`self.Camera1`) false))

(fn `IsHoldingObject`
  (returns (bIsHoldingObject :type Boolean))
  (return (!= (`self.HeldObject`) null)))

(fn `UserConstructionScript`)