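; Runs a timed round of randomly generated office chores (copy, fax, tube, file, shred), counting successes and fails and showing an end screen when time expires.
; A randomly delayed loop fills free task slots, mirrored in W_TaskList, whose widgets hold each task's timer.
; Machine messages clear the matching task with least time left, while TaskFailed counts failures.
; Tick pushes round time and tallies to the HUD; StartDay's announcement is never called here.
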(event `self.ReceiveTick`
  (params (DeltaSeconds :type "Float (single-precision)"))
  (bind _roundtimerfailcounter (`self.RoundTimerFailCounter`))
  (set `/Game/MyContent/Blueprints/WorkingTaskWidgets/W_RoundTimerAndFailCounter.RoundTimeRemaining` (`KismetSystemLibrary.K2_GetTimerRemainingTimeHandle` (`self.RoundTimer`)) _roundtimerfailcounter)
  (set `/Game/MyContent/Blueprints/WorkingTaskWidgets/W_RoundTimerAndFailCounter.Fails` (`self.NumberOfFails`) _roundtimerfailcounter)
  (set `/Game/MyContent/Blueprints/WorkingTaskWidgets/W_RoundTimerAndFailCounter.Successes` (`self.NumberOfSuccesses`) _roundtimerfailcounter))

(event `StartRound`
  (bind _returnvalue (`KismetSystemLibrary.K2_SetTimerDelegate` (delegate `EndRound`) (`self.RoundDuration`)))
  (set `self.RoundTimer` _returnvalue)
  (`KismetSystemLibrary.Delay` 2.0)
  (`self.GenerateTask` :!label _label)
  (`KismetSystemLibrary.Delay` (`KismetMathLibrary.RandomFloatInRange` (`self.MinDelayBeforeNextTask`) (`self.MaxDelayBeforeNextTask`)))
  (goto _label))

(event `EndRound`
  (bind _returnvalue (`|CreateWidget` "/Game/MyContent/Blueprints/W_EndScreen.W_EndScreen_C"))
  (`UserWidget.AddToViewport` _returnvalue 0))

(event `GenerateTask`
  ;[1 1 1] Set tasks here. Send status to widgets. Timers located in task widget.
  (`self.AddRandomTask`) ; Adds in correct spot if one is available
)

(event `Key|R`
  (params (Key :type "Key Structure"))
  ;[1 0 0] Testing
)

(event `self.ReceiveBeginPlay`
  (bind _maxtasks (`self.MaxTasks`))
  ;[1 1 1 1 24] TaskListWidget holds and displays the tasks
  (bind _returnvalue (`|CreateWidget` "/Game/MyContent/Blueprints/WorkingTaskWidgets/W_TaskList.W_TaskList_C" (`GameplayStatics.GetPlayerController` 0)))
  (set `self.TaskListWidget` _returnvalue)
  (`UserWidget.AddToViewport` _returnvalue 0)
  ;;[1 1 1] Sets up task containers
  (`/Game/MyContent/Blueprints/WorkingTaskWidgets/W_TaskList.Initialize` _returnvalue _maxtasks self)
  ;;[1 1 1] Initialize tasks to none
  (for _ (range _maxtasks)
    (`KismetArrayLibrary.Array_Add` (`self.Tasks`) "NewEnumerator10"))
  (`self.InitializeRoundTimerFailCounter`)
  (`self.StartRound`))

(event `StartDay`
  (bind _announcementwidget (`self.AnnouncementWidget`))
  ;[1 0 0] Maybe someday I'll get around to implementing this
  (bind _returnvalue (`|CreateWidget` "/Game/MyContent/Blueprints/W_Announcement.W_Announcement_C" (`GameplayStatics.GetPlayerController` 0)))
  (set `self.AnnouncementWidget` _returnvalue)
  (`UserWidget.AddToViewport` _announcementwidget 0)
  (`/Game/MyContent/Blueprints/W_Announcement.Announce` _announcementwidget "The Boss" "Alllllllllllright team! It's time for our daily morale chant! Get into position!" 10.0))

(event `Message`
  (params (SenderActorClass :type "Actor Class Reference"))
  ;[1 1 1 1 32] Message from machines to task manager
  ;;[1 1 1] Tube
  (if (== SenderActorClass "/Game/MyContent/Blueprints/PlayerProps/BP_Interactable_Tube.BP_Interactable_Tube_C")
    ;;[1 1 1] Tube message sent
    (`self.RemoveTask` "NewEnumerator2")
    (else
      ;;[1 1 1] Shred
      (if (== SenderActorClass "/Game/MyContent/Blueprints/PlayerProps/BP_InteractableShredder.BP_InteractableShredder_C")
        ;;[1 1 1] Report Shredded
        (`self.RemoveTask` "NewEnumerator7")
        (else
          ;;[1 1 1] Fax
          (if (== SenderActorClass "/Game/MyContent/Blueprints/PlayerProps/BP_Interactable_Fax.BP_Interactable_Fax_C")
            ;;[1 1 1] Report Faxed
            (`self.RemoveTask` "NewEnumerator1")
            (else
              ;;[1 1 1] Filing
              (if (== SenderActorClass "/Game/MyContent/Blueprints/PlayerProps/BP_InteractableFilingCabinet.BP_InteractableFilingCabinet_C")
                ;;[1 1 1] Report FIled
                (`self.RemoveTask` "NewEnumerator6")
                (else
                  ;;[1 1 1] Copier
                  (if (== SenderActorClass "/Game/MyContent/Blueprints/PlayerProps/BP_Interactable_Copier.BP_Interactable_Copier_C")
                    ;;[1 1 1] Report Copied
                    (`self.RemoveTask` "NewEnumerator9")))))))))))

(fn `AddRandomTask`
  (returns (bSuccess :type Boolean) (Index :type Integer))
  (locals (bSuccessful :type Boolean))
  (bind _tasks (`self.Tasks`))
  (set `local.bSuccessful` false)
  (for _index (range (`self.MaxTasks`))
    (switch `/Game/MyContent/Blueprints/E_Task` (`|GetArrayItem` _tasks _index)
      (:`NewEnumerator10`
        (bind _newtask (`self.HelperRandomTask`))
        (`KismetArrayLibrary.Array_Set` _tasks _index _newtask)
        ;[1 1 1] Notify TaskList widget
        (`/Game/MyContent/Blueprints/WorkingTaskWidgets/W_TaskList.AddTask` (`self.TaskListWidget`) _index _newtask (`self.TaskTimeDuration`))
        (set `local.bSuccessful` true)
        (break))))
  (return (`local.bSuccessful`) _index))

(fn `HelperRandomTask`
  (returns (NewTask :type "/Game/MyContent/Blueprints/E_Task Enum"))
  (switch `int` (`KismetMathLibrary.RandomIntegerInRange` 0 4)
    (:`Default`
      _)
    (:`0`
      (return "NewEnumerator1"))
    (:`1`
      (return "NewEnumerator2"))
    (:`2`
      (return "NewEnumerator6"))
    (:`3`
      (return "NewEnumerator7"))
    (:`4`
      _))
  (return "NewEnumerator9"))

(fn `InitializeRoundTimerFailCounter`
  (bind _returnvalue (`|CreateWidget` "/Game/MyContent/Blueprints/WorkingTaskWidgets/W_RoundTimerAndFailCounter.W_RoundTimerAndFailCounter_C"))
  (`UserWidget.AddToViewport` _returnvalue 0)
  (set `self.RoundTimerFailCounter` _returnvalue))

(fn `RemoveTask`
  (params (TaskToRemove :type "/Game/MyContent/Blueprints/E_Task Enum" :default "NewEnumerator10"))
  (returns (bSuccess :type Boolean))
  (locals (bIsSuccessful :type Boolean) (TimesRemaining :type "Array of Float (double-precision)"))
  (bind (_indexofminvalue _minvalue) (`KismetMathLibrary.MinOfFloatArray` (`local.TimesRemaining`)))
  (for _ (range (`self.MaxTasks`))
    (`KismetArrayLibrary.Array_Add` (`local.TimesRemaining`) 1000000.0))
  ;[1 1 1] Cycle through tasks
  (for (_array_element _array_index) (`self.Tasks`)
    ;[1 1 1] Get all of the corresponding tasks
    (if (`|EnumEquality` TaskToRemove _array_element)
      (bind _timeremaining (`/Game/MyContent/Blueprints/WorkingTaskWidgets/W_NewTaskBG.GetTimeRemaining` (`|GetArrayItem` (`/Game/MyContent/Blueprints/WorkingTaskWidgets/W_TaskList.TaskBGWidgets` (`self.TaskListWidget`)) _array_index)))
      (`KismetArrayLibrary.Array_Set` (`local.TimesRemaining`) _array_index _timeremaining)))
  ;[1 1 1] Take away lowest time remaining
  (if (< _minvalue 1000000.0)
    (`self.SetTask` _indexofminvalue "NewEnumerator10" 0.0)
    (set `local.bIsSuccessful` true)
    (`/Engine/EditorBlueprintResources/StandardMacros.IncrementInt` (`self.NumberOfSuccesses`)
      (:`  `
        _)))
  (return (`local.bIsSuccessful`)))

(fn `SetTask`
  (params (Index :type Integer) (NewTask :type "/Game/MyContent/Blueprints/E_Task Enum" :default "NewEnumerator10") (TaskDuration :type "Float (double-precision)"))
  (`KismetArrayLibrary.Array_Set` (`self.Tasks`) Index NewTask)
  (`/Game/MyContent/Blueprints/WorkingTaskWidgets/W_TaskList.UpdateTask` (`self.TaskListWidget`) Index NewTask TaskDuration))

(fn `TaskFailed`
  (params (Index :type Integer))
  (`/Engine/EditorBlueprintResources/StandardMacros.IncrementInt` (`self.NumberOfFails`)
    (:`  `
      (`self.SetTask` Index))))

(fn `UserConstructionScript`)