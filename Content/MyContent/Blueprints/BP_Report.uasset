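; BP_Report is a report item that the BP_OfficeGuy character can pick up with the Use action.
; A sphere overlap stores the character and enables player 0 input on the actor, and leaving clears both.
; On Use, if the character's HeldObject is empty, it passes its own class to PickupObject and destroys itself.
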(event `InputAction|Use`
  (params (Key :type "Key Structure"))
  (bind _char (`self.Char`))
  (:`Pressed`
    (`/Engine/EditorBlueprintResources/StandardMacros.IsValid` _char
      (:`Is Valid`
        (if (== (`/Game/MyContent/Blueprints/OfficeGuy/BP_OfficeGuy.HeldObject` _char) null)
          (`/Game/MyContent/Blueprints/OfficeGuy/BP_OfficeGuy.PickupObject` _char (`GameplayStatics.GetObjectClass` self))
          (`self.K2_DestroyActor`))))))

(event `self.Sphere.OnComponentBeginOverlap`
  (params (OverlappedComponent :type "PrimitiveComponent Object Reference") (OtherActor :type "Actor Object Reference") (OtherComp :type "PrimitiveComponent Object Reference") (OtherBodyIndex :type Integer) (bFromSweep :type Boolean) (SweepResult :type "HitResult Structure (by ref)"))
  (bind _asbp_office_guy (cast `/Game/MyContent/Blueprints/OfficeGuy/BP_OfficeGuy` OtherActor))
  (set `self.Char` _asbp_office_guy)
  (`self.EnableInput` (`GameplayStatics.GetPlayerController` 0)))

(event `self.Sphere.OnComponentEndOverlap`
  (params (OverlappedComponent :type "PrimitiveComponent Object Reference") (OtherActor :type "Actor Object Reference") (OtherComp :type "PrimitiveComponent Object Reference") (OtherBodyIndex :type Integer))
  (cast `/Game/MyContent/Blueprints/OfficeGuy/BP_OfficeGuy` OtherActor)
  ;[1 1 1] Clear
  (set `self.Char` null)
  (`self.DisableInput` (`GameplayStatics.GetPlayerController` 0)))

(fn `UserConstructionScript`)