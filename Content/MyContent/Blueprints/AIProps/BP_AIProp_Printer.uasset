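; BP_AIProp_Printer is an AI prop for a printer that animates paper coming out when its action is performed.
; PerformAction calls the parent, then plays a timeline that lerps the PaperOut component's relative transform from its initial to its final value.
; One second after the timeline finishes, the paper snaps back to its initial transform.
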(event `self.PerformAction`
  (`parent.PerformAction`)
  (bind (_direction _alpha) (`Timeline|Timeline_0` :!via `PlayFromStart`)
    (:`Update`
      (`SceneComponent.K2_SetRelativeTransform` (`self.PaperOut`) (`KismetMathLibrary.TLerp` (`self.PaperOutInitTrans`) (`self.PaperOutFinalTrans`) _alpha) false false))
    (:`Finished`
      (`KismetSystemLibrary.Delay` 1.0)
      (`SceneComponent.K2_SetRelativeTransform` (`self.PaperOut`) (`self.PaperOutInitTrans`) false false))))

(fn `UserConstructionScript`
  (`parent.UserConstructionScript`))