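; BP_AIProp_Copier is a copier prop, named as an AI prop, whose top mesh swings open and shut as an action starts and stops.
; BeginPlay caches the top mesh's initial relative rotation.
; PerformAction plays the ActionDriver timeline, whose alpha lerps the mesh from that rotation to a fixed roll offset.
; StopAction reverses the same timeline to return it.
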(event `self.PerformAction`
  (bind _topinitrot (`self.TopInitRot`))
  (bind (_direction _alpha) (`Timeline|ActionDriver` :!label _label)
    (:`Update`
      (`SceneComponent.K2_SetRelativeRotation` (`self.StaticMesh1`) (`KismetMathLibrary.RLerp` _topinitrot (`KismetMathLibrary.MakeRotator` (+ (.roll _topinitrot) -75.0) (.pitch _topinitrot) (.yaw _topinitrot)) _alpha) false false))))

(event `self.StopAction`
  (goto _label :!via `Reverse`))

(event `self.ReceiveBeginPlay`
  (set `self.TopInitRot` (`SceneComponent.RelativeRotation` (`self.StaticMesh1`))))

(fn `UserConstructionScript`
  (`parent.UserConstructionScript`))