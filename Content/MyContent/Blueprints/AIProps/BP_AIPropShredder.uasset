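; BP_AIPropShredder is a shredder AI prop that animates a sheet of paper when its PerformAction event fires.
; A timeline lerps the Paper component's relative location from its initial to its final position, then snaps it to the final position on finish.
; A DoOnce gate ignores repeat calls during playback and resets when the timeline completes, so each later action replays the motion from the start.
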(event `self.PerformAction`
  (bind _paperfinalloc (`self.PaperFinalLoc`))
  (`/Engine/EditorBlueprintResources/StandardMacros.DoOnce` false :!label _label
    (:`Completed`
      (bind (_direction _alpha) (`Timeline|Timeline_0` :!via `PlayFromStart`)
        (:`Update`
          (`SceneComponent.K2_SetRelativeLocation` (`self.Paper`) (`KismetMathLibrary.VLerp` (`self.PaperInitLoc`) _paperfinalloc _alpha) false false))
        (:`Finished`
          (`SceneComponent.K2_SetRelativeLocation` (`self.Paper`) _paperfinalloc false false)
          (goto _label :!via `Reset`))))))

(fn `UserConstructionScript`
  (`parent.UserConstructionScript`))