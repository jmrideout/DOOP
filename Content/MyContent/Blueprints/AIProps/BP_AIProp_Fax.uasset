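; BP_AIProp_Fax is a fax machine AI prop that animates paper feeding in and out when its action is performed.
; PerformAction plays the FaxDriver timeline, whose two alphas lerp the PaperIn and PaperOut relative transforms between their initial and final poses.
; On completion, StopAction waits briefly, then calls ResetPaper, also run at BeginPlay, which sets PaperIn to its final pose and PaperOut to its initial one.
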(event `self.PerformAction`
  (bind (_direction _paperinalpha _paperoutalpha) (`Timeline|FaxDriver`)
    (:`Update`
      (`SceneComponent.K2_SetRelativeTransform` (`self.PaperIn`) (`KismetMathLibrary.TLerp` (`self.PaperInInitTransform`) (`self.PaperInFinalTransform`) _paperinalpha) false false)
      (`SceneComponent.K2_SetRelativeTransform` (`self.PaperOut`) (`KismetMathLibrary.TLerp` (`self.PaperOutInitTransform`) (`self.PaperOutFinalTransform`) _paperoutalpha) false false))
    (:`Complete`
      (`self.StopAction`))))

(event `self.StopAction`
  (`KismetSystemLibrary.Delay` 1.0)
  (`self.ResetPaper`))

(event `ResetPaper`
  (`SceneComponent.K2_SetRelativeTransform` (`self.PaperIn`) (`self.PaperInFinalTransform`) false false)
  (`SceneComponent.K2_SetRelativeTransform` (`self.PaperOut`) (`self.PaperOutInitTransform`) false false))

(event `self.ReceiveBeginPlay`
  (`self.ResetPaper`))

(fn `UserConstructionScript`
  (`parent.UserConstructionScript`))