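; An interactable paper shredder prop that animates a sheet of paper and reports to the task manager when the action completes.
; It extends a parent interactable, setting the meter widget's label to shredding on begin play.
; Its animation override triggers the character's use-object action while a timeline lerps the paper between initial and final transforms.
; On completion it messages the task manager with its own class.
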(event `self.BlueprintSpecificAnimation`
  ;[1 1 1] Animation
  (`parent.BlueprintSpecificAnimation`)
  (`/Game/MyContent/Blueprints/OfficeGuy/BP_OfficeGuy.UseObject` (`self.Char`))
  (bind (_direction _alpha) (`Timeline|AnimationDriver` :!via `PlayFromStart`)
    (:`Update`
      (`SceneComponent.K2_SetRelativeTransform` (`self.Paper`) (`KismetMathLibrary.TLerp` (`self.PaperInitTrans`) (`self.PaperFinalTrans`) _alpha) false false))
    (:`Finished`
      (`SceneComponent.K2_SetRelativeTransform` (`self.Paper`) (`self.PaperFinalTrans`) false false))))

(event `self.ReceiveBeginPlay`
  (`parent.ReceiveBeginPlay`)
  (bind _asw_meter (cast `/Game/MyContent/Blueprints/W_Meter` (`WidgetComponent.GetUserWidgetObject` (`self.MeterWidget`))))
  (set `/Game/MyContent/Blueprints/W_Meter.MeterText` "Shredding..." _asw_meter))

(event `self.CompleteAction`
  (`parent.CompleteAction`)
  (`/Game/MyContent/Blueprints/BP_TaskManager.Message` (`self.TaskManager`) (`GameplayStatics.GetObjectClass` self)))

(fn `UserConstructionScript`
  (`parent.UserConstructionScript`))