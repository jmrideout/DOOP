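; BP_InteractablePrinter is an interactable printer prop that prints a report when its action is started by a computer rather than by player overlap.
; A timeline animates the paper sliding out, then spawns a BP_Report in its place and resets the paper mesh.
; Completing the action notifies the TaskManager.
; Tick watches the spawned report and resets the attached computer once that report is no longer valid, treated as picked up.
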(event `self.CompleteAction`
  (`parent.CompleteAction`)
  (`/Game/MyContent/Blueprints/BP_TaskManager.Message` (`self.TaskManager`) (`GameplayStatics.GetObjectClass` self)))

(event `self.PerformAction`
  (`parent.PerformAction`))

(event `self.BlueprintSpecificAnimation`
  (bind (_direction _alpha) (`Timeline|AnimationDriver` :!via `PlayFromStart`)
    (:`Update`
      (`SceneComponent.K2_SetRelativeTransform` (`self.PaperOut`) (`KismetMathLibrary.TLerp` (`self.PaperOutInitTrans`) (`self.PaperOutFinalTrans`) _alpha) false false))
    (:`Finished`
      (bind _returnvalue (`|SpawnActorFromClass` "/Game/MyContent/Blueprints/BP_Report.BP_Report_C" (`KismetMathLibrary.MakeTransform` (.location (`SceneComponent.K2_GetComponentToWorld` (`self.PaperOut`))) (.rotation (`SceneComponent.K2_GetComponentToWorld` (`self.PaperOut`)))) "AlwaysSpawn" "OverrideRootScale" null null))
      (set `self.TheReport` _returnvalue)
      (`SceneComponent.K2_SetRelativeTransform` (`self.PaperOut`) (`self.PaperOutInitTrans`) false false)
      (set `self.bHasPaper` true))))

(event `self.ReceiveBeginPlay`
  (`parent.ReceiveBeginPlay`)
  (bind _asw_meter (cast `/Game/MyContent/Blueprints/W_Meter` (`WidgetComponent.GetUserWidgetObject` (`self.MeterWidget`))))
  (set `/Game/MyContent/Blueprints/W_Meter.MeterText` "Printing..." _asw_meter))

(event `self.ReceiveTick`
  (params (DeltaSeconds :type "Float (single-precision)"))
  (`parent.ReceiveTick` DeltaSeconds)
  ;[1 1 1] The paper has been printed
  (if (`self.bHasPaper`)
    ;[1 1 1] The paper has been picked up
    (`/Engine/EditorBlueprintResources/StandardMacros.IsValid` (`self.TheReport`)
      (:`Is Not Valid`
        (set `self.bHasPaper` false)
        (`/Game/MyContent/Blueprints/PlayerProps/BP_Interactable_Desk.Reset` (`self.AttachedComputer`))))))

(event `self.Box.OnComponentBeginOverlap`
  (params (OverlappedComponent :type "PrimitiveComponent Object Reference") (OtherActor :type "Actor Object Reference") (OtherComp :type "PrimitiveComponent Object Reference") (OtherBodyIndex :type Integer) (bFromSweep :type Boolean) (SweepResult :type "HitResult Structure (by ref)"))
  ;[1 1 1] Override to do nothing. Action is initiated by computer
)

(event `self.Box.OnComponentEndOverlap`
  (params (OverlappedComponent :type "PrimitiveComponent Object Reference") (OtherActor :type "Actor Object Reference") (OtherComp :type "PrimitiveComponent Object Reference") (OtherBodyIndex :type Integer))
  ;[1 1 1] Override to do nothing. Action is initiated by computer
)

(fn `UserConstructionScript`
  (`parent.UserConstructionScript`))