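; Base interactable prop that BP_OfficeGuy uses through the Use input while overlapping its box.
; Use checks readiness, empty-hand and required-object conditions, consumes any required item, then starts or resumes a timed action with a meter widget.
; Leaving the box pauses the timer if presence is required.
; Alert shows an indicator that Tick bobs on a sine wave, and children override BlueprintSpecificAnimation for their own animation.
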(event `Alert`
  (params (AlertIcon :type "Object Object Reference"))
  (set `self.AlertIcon` AlertIcon)
  (set `self.bHasAlert` true)
  (bind _asw_indicator (cast `/Game/MyContent/Blueprints/W_Indicator` (`WidgetComponent.GetUserWidgetObject` (`self.IndicatorWidget`))))
  (set `/Game/MyContent/Blueprints/W_Indicator.bIsVisible` true _asw_indicator))

(event `InputAction|Use` :consume false
  (params (Key :type "Key Structure"))
  (bind _char (`self.Char`))
  (:`Pressed`
    (if (`self.bIsReady`)
      (`/Engine/EditorBlueprintResources/StandardMacros.IsValid` (`self.Char`)
        (:`Is Valid`
          (if (`self.bMustBeEmptyHanded`)
            (bind _bisholdingobject (`/Game/MyContent/Blueprints/OfficeGuy/BP_OfficeGuy.IsHoldingObject` (`self.Char`)))
            (if (not _bisholdingobject)
              ;[1 1 1] If no required object
              (if (== (`self.RequiredObject`) null) :!label _label
                (`self.PerformAction`)
                (else
                  ;[1 1 1] If player is holding required object, remove object and perform action
                  (if (== (`/Game/MyContent/Blueprints/OfficeGuy/BP_OfficeGuy.HeldObject` _char) (`self.RequiredObject`))
                    (set `/Game/MyContent/Blueprints/OfficeGuy/BP_OfficeGuy.HeldObject` null _char)
                    (`self.PerformAction`)))))
            (else
              (goto _label))))))))

(event `BlueprintSpecificAnimation`
  ;[1 1 1] To be overridden in children
)

(event `self.ReceiveBeginPlay`
  ;[1 1 1] Initialize
  (set `self.IndicatorInitLoc` (`SceneComponent.RelativeLocation` (`self.IndicatorWidget`)))
  (bind _asw_indicator (cast `/Game/MyContent/Blueprints/W_Indicator` (`WidgetComponent.GetUserWidgetObject` (`self.IndicatorWidget`))))
  (set `/Game/MyContent/Blueprints/W_Indicator.AlertImage` (`self.AlertIcon`) _asw_indicator))

(event `self.ReceiveTick`
  (params (DeltaSeconds :type "Float (single-precision)"))
  (bind _actiontimer (`self.ActionTimer`))
  (bind _returnvalue (`KismetSystemLibrary.K2_GetTimerRemainingTimeHandle` _actiontimer))
  (`|ExecutionSequence`
    (:`then_0`
      ;[1 1 1] Meter
      (if (> (`self.ActionDuration`) 0.1)
        (if (`self.bIsInUse`)
          (if (`KismetSystemLibrary.K2_IsValidTimerHandle` _actiontimer)
            (bind _asw_meter (cast `/Game/MyContent/Blueprints/W_Meter` (`WidgetComponent.GetUserWidgetObject` (`self.MeterWidget`))))
            (`/Game/MyContent/Blueprints/W_Meter.SetPercentComplete` _asw_meter (/ _returnvalue (+ _returnvalue (`KismetSystemLibrary.K2_GetTimerElapsedTimeHandle` _actiontimer))))))))
    (:`then_1`
      (if (`self.bHasAlert`)
        (`self.BobAlert`)))))

(event `self.Box.OnComponentBeginOverlap`
  (params (OverlappedComponent :type "PrimitiveComponent Object Reference") (OtherActor :type "Actor Object Reference") (OtherComp :type "PrimitiveComponent Object Reference") (OtherBodyIndex :type Integer) (bFromSweep :type Boolean) (SweepResult :type "HitResult Structure (by ref)"))
  ;[1 1 1] Overlaps
  (bind _asbp_office_guy (cast `/Game/MyContent/Blueprints/OfficeGuy/BP_OfficeGuy` OtherActor))
  (set `self.Char` _asbp_office_guy)
  (`self.EnableInput` (`GameplayStatics.GetPlayerController` 0)))

(event `self.Box.OnComponentEndOverlap`
  (params (OverlappedComponent :type "PrimitiveComponent Object Reference") (OtherActor :type "Actor Object Reference") (OtherComp :type "PrimitiveComponent Object Reference") (OtherBodyIndex :type Integer))
  (bind _actiontimer (`self.ActionTimer`))
  ;[1 1 1] Overlaps
  (cast `/Game/MyContent/Blueprints/OfficeGuy/BP_OfficeGuy` OtherActor)
  (`self.DisableInput` (`GameplayStatics.GetPlayerController` 0))
  (if (`KismetSystemLibrary.K2_IsValidTimerHandle` _actiontimer)
    (if (`self.bMustBePresent`)
      (`KismetSystemLibrary.K2_PauseTimerHandle` _actiontimer))))

(fn `BobAlert`
  (set `self.CurrentTime` (+ (`self.CurrentTime`) (`GameplayStatics.GetWorldDeltaSeconds`)))
  (`SceneComponent.K2_SetRelativeLocation` (`self.IndicatorWidget`) (+ (* (`self.VerticalBobDisplacement`) (`KismetMathLibrary.DegSin` (* (`self.CurrentTime`) (`self.IndicatorBobRate`) 360.0))) (`self.IndicatorInitLoc`)) false false))

(fn `CompleteAction`
  (set `self.bIsInUse` false)
  (`KismetSystemLibrary.K2_ClearAndInvalidateTimerHandle` (`self.ActionTimer`))
  (bind _asw_meter (cast `/Game/MyContent/Blueprints/W_Meter` (`WidgetComponent.GetUserWidgetObject` (`self.MeterWidget`))))
  (set `/Game/MyContent/Blueprints/W_Meter.MeterVisibility` "Hidden" _asw_meter))

(fn `PerformAction`
  (set `self.bIsInUse` true)
  (if (`KismetSystemLibrary.K2_IsValidTimerHandle` (`self.ActionTimer`))
    (`KismetSystemLibrary.K2_UnPauseTimerHandle` (`self.ActionTimer`))
    (else
      (bind _returnvalue (`KismetSystemLibrary.K2_SetTimer` null "CompleteAction" (`self.ActionDuration`)))
      (set `self.ActionTimer` _returnvalue)
      (`self.BlueprintSpecificAnimation`)
      (if (> (`self.ActionDuration`) 0.1)
        (bind _asw_meter (cast `/Game/MyContent/Blueprints/W_Meter` (`WidgetComponent.GetUserWidgetObject` (`self.MeterWidget`))))
        (set `/Game/MyContent/Blueprints/W_Meter.MeterVisibility` "Visible" _asw_meter)))))

(fn `UserConstructionScript`)