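; Interactable desk prop with a computer, where the player performs a typing action that feeds a connected printer.
; During the action animation, the monitor switches to a screen material, with a small random chance of a capture material instead.
; Completion triggers the printer, restores the monitor, reports to the task manager and locks the desk until a Reset, intended to come from the printer.
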(event `self.BlueprintSpecificAnimation`
  (bind _computer (`self.Computer`))
  ;[1 1 1] Animation
  (`parent.BlueprintSpecificAnimation`)
  (if (< (`KismetMathLibrary.RandomFloatInRange` 0.0 100.0) 10.0)
    (`PrimitiveComponent.SetMaterialByName` _computer "MonitorScreen" "/Game/MyContent/Materials/M_Capture.M_Capture")
    (else
      (`PrimitiveComponent.SetMaterialByName` _computer "MonitorScreen" "/Game/MyContent/Materials/M_Screen.M_Screen"))))

(event `self.CompleteAction`
  ;[1 1 1] Complete action
  (`parent.CompleteAction`)
  (`self.PerformAction` (`self.ConnectedPrinter`))
  (`PrimitiveComponent.SetMaterialByName` (`self.Computer`) "MonitorScreen" "/Game/MyContent/Materials/MonitorScreen.MonitorScreen")
  (set `self.bIsReady` false)
  (`/Game/MyContent/Blueprints/BP_TaskManager.Message` (`self.TaskManager`) (`GameplayStatics.GetObjectClass` self)))

(event `Reset`
  ;[1 1 1] Must get the signal from printer
  (set `self.bIsReady` true))

(event `self.PerformAction`
  (`parent.PerformAction`))

(event `self.ReceiveBeginPlay`
  ;[1 1 1] Begin Play
  (`parent.ReceiveBeginPlay`)
  (bind _asw_meter (cast `/Game/MyContent/Blueprints/W_Meter` (`WidgetComponent.GetUserWidgetObject` (`self.MeterWidget`))))
  (set `/Game/MyContent/Blueprints/W_Meter.MeterText` "Typing..." _asw_meter))

(fn `UserConstructionScript`
  (`parent.UserConstructionScript`))