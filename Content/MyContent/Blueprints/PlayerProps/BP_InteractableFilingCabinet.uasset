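; An interactable filing cabinet prop, built on a parent interactable class, that serves as a "Filing..." task for the player.
; BlueprintSpecificAnimation plays a timeline that lerps the top and bottom drawers open on separate alpha tracks.
; On completion it reverses that timeline to close them, calls UseObject on the character and messages the task manager with its class.
; BeginPlay sets the label on its widget meter.
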(event `self.CompleteAction`
  (`parent.CompleteAction`)
  (`/Game/MyContent/Blueprints/OfficeGuy/BP_OfficeGuy.UseObject` (`self.Char`))
  (`/Game/MyContent/Blueprints/BP_TaskManager.Message` (`self.TaskManager`) (`GameplayStatics.GetObjectClass` self))
  (bind (_direction _alphatop _alphabottom) (`Timeline|AnimationDriver` :!via `ReverseFromEnd` :!label _label)
    (:`Update`
      (`SceneComponent.K2_SetRelativeLocation` (`self.TopDrawer`) (`KismetMathLibrary.VLerp` (0.0 0.0 0.0) (0.0 30.0 0.0) _alphatop) false false)
      (`SceneComponent.K2_SetRelativeLocation` (`self.BottomDrawer`) (`KismetMathLibrary.VLerp` (0.0 0.0 0.0) (0.0 40.0 0.0) _alphabottom) false false))))

(event `self.PerformAction`
  (`parent.PerformAction`))

(event `self.BlueprintSpecificAnimation`
  (goto _label :!via `PlayFromStart`))

(event `self.ReceiveBeginPlay`
  (`parent.ReceiveBeginPlay`)
  (bind _asw_meter (cast `/Game/MyContent/Blueprints/W_Meter` (`WidgetComponent.GetUserWidgetObject` (`self.MeterWidget`))))
  (set `/Game/MyContent/Blueprints/W_Meter.MeterText` "Filing..." _asw_meter))

(fn `UserConstructionScript`
  (`parent.UserConstructionScript`))