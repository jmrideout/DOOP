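; Interactable fax machine prop that the character uses to produce a report, extending a parent interactable with a "Faxing..." meter.
; Use is allowed only while no valid report from this machine exists, and completing the action messages the TaskManager with the fax's class.
; A timeline slides the in and out paper meshes between stored transforms, then spawns a BP_Report at the output paper and resets that paper.
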(event `self.PerformAction`
  (`/Engine/EditorBlueprintResources/StandardMacros.IsValid` (`self.TheReport`)
    (:`Is Not Valid`
      (`parent.PerformAction`)
      (`/Game/MyContent/Blueprints/OfficeGuy/BP_OfficeGuy.UseObject` (`self.Char`)))))

(event `self.CompleteAction`
  (`parent.CompleteAction`)
  (`/Game/MyContent/Blueprints/BP_TaskManager.Message` (`self.TaskManager`) (`GameplayStatics.GetObjectClass` self)))

(event `self.BlueprintSpecificAnimation`
  (bind (_direction _paperinalpha _paperoutalpha) (`Timeline|AnimationDriver` :!via `PlayFromStart`)
    (:`Update`
      (`SceneComponent.K2_SetRelativeTransform` (`self.PaperIn`) (`KismetMathLibrary.TLerp` (`self.PaperInInitTransform`) (`self.PaperInFinalTransform`) _paperinalpha) false false)
      (`SceneComponent.K2_SetRelativeTransform` (`self.PaperOut`) (`KismetMathLibrary.TLerp` (`self.PaperOutInitTransform`) (`self.PaperOutFinalTransform`) _paperoutalpha) false false))
    (:`Finished`
      (bind _returnvalue (`|SpawnActorFromClass` "/Game/MyContent/Blueprints/BP_Report.BP_Report_C" (`KismetMathLibrary.MakeTransform` (.location (`SceneComponent.K2_GetComponentToWorld` (`self.PaperOut`))) (.rotation (`SceneComponent.K2_GetComponentToWorld` (`self.PaperOut`)))) "AlwaysSpawn" "OverrideRootScale" null null))
      (set `self.TheReport` _returnvalue)
      (`SceneComponent.K2_SetRelativeTransform` (`self.PaperOut`) (`self.PaperOutInitTransform`) false false))))

(event `ResetPaper`
  (`SceneComponent.K2_SetRelativeTransform` (`self.PaperIn`) (`self.PaperInFinalTransform`) false false)
  (`SceneComponent.K2_SetRelativeTransform` (`self.PaperOut`) (`self.PaperOutInitTransform`) false false))

(event `self.ReceiveBeginPlay`
  (`parent.ReceiveBeginPlay`)
  (`self.ResetPaper`)
  (bind _asw_meter (cast `/Game/MyContent/Blueprints/W_Meter` (`WidgetComponent.GetUserWidgetObject` (`self.MeterWidget`))))
  (set `/Game/MyContent/Blueprints/W_Meter.MeterText` "Faxing..." _asw_meter))

(fn `UserConstructionScript`
  (`parent.UserConstructionScript`))