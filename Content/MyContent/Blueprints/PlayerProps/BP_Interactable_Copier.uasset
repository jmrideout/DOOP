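; BP_Interactable_Copier is an interactable office copier prop whose lid animates during the player's interaction.
; It overrides the parent's BlueprintSpecificAnimation event to play a timeline that rotates the Lid component open.
; CompleteAction runs the parent logic, sends the copier's class to TaskManager as a message, then reverses the timeline to close the lid.
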(event `self.BlueprintSpecificAnimation`
  (bind (_direction _alpha) (`Timeline|Timeline_0` :!via `PlayFromStart` :!label _label)
    (:`Update`
      (`SceneComponent.K2_SetRelativeRotation` (`self.Lid`) (`KismetMathLibrary.RLerp` (struct) (struct :`Roll` -75.0) _alpha) false false))))

(event `self.CompleteAction`
  (`parent.CompleteAction`)
  (`/Game/MyContent/Blueprints/BP_TaskManager.Message` (`self.TaskManager`) (`GameplayStatics.GetObjectClass` self))
  (goto _label :!via `ReverseFromEnd`))

(fn `UserConstructionScript`
  (`parent.UserConstructionScript`))