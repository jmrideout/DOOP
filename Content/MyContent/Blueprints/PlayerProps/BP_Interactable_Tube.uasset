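; Interactable tube prop that the player uses to perform a "sending" task, built on a parent interactable Blueprint.
; BeginPlay labels the meter widget "Sending...", and performing the action makes the character use the object.
; Completing the action reports the prop's class to the TaskManager.
; Its specific animation hook plays a timeline that lerps the mesh's relative rotation to a 90-degree turn.
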(event `self.CompleteAction`
  (`parent.CompleteAction`)
  (`/Game/MyContent/Blueprints/BP_TaskManager.Message` (`self.TaskManager`) (`GameplayStatics.GetObjectClass` self)))

(event `self.PerformAction`
  (`parent.PerformAction`)
  (`/Game/MyContent/Blueprints/OfficeGuy/BP_OfficeGuy.UseObject` (`self.Char`)))

(event `self.BlueprintSpecificAnimation`
  (bind (_direction _alpha) (`Timeline|AnimDriver` :!via `PlayFromStart`)
    (:`Update`
      (`SceneComponent.K2_SetRelativeRotation` (`self.StaticMesh1`) (`KismetMathLibrary.RLerp` (struct) (struct :`Yaw` 90.0) _alpha) false false))))

(event `self.ReceiveBeginPlay`
  (`parent.ReceiveBeginPlay`)
  (bind _asw_meter (cast `/Game/MyContent/Blueprints/W_Meter` (`WidgetComponent.GetUserWidgetObject` (`self.MeterWidget`))))
  (set `/Game/MyContent/Blueprints/W_Meter.MeterText` "Sending..." _asw_meter))

(fn `UserConstructionScript`
  (`parent.UserConstructionScript`))