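; OfficeAI is an office worker character that uses AI props it bumps into.
; On actor overlap it takes the first component overlapping its capsule and, if that is a box owned by a BP_AIPropBase, calls that prop's PerformAction.
; It then disables movement, plays a one-shot use animation, and after a short delay restores walking and Animation Blueprint mode.
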(event `self.ReceiveActorBeginOverlap`
  (params (OtherActor :type "Actor Object Reference"))
  (bind _asbox_collision (cast `BoxComponent` (`|GetArrayItem` (`PrimitiveComponent.GetOverlappingComponents` (`self.CapsuleComponent`)))))
  (bind _asbp_aiprop_base (cast `/Game/MyContent/Blueprints/AIProps/BP_AIPropBase` (`ActorComponent.GetOwner` _asbox_collision)))
  (`/Game/MyContent/Blueprints/AIProps/BP_AIPropBase.PerformAction` _asbp_aiprop_base)
  (`CharacterMovementComponent.SetMovementMode` (`self.CharacterMovement`) "MOVE_None" 0)
  (`SkeletalMeshComponent.PlayAnimation` (`self.Mesh`) "/Game/MyContent/Blueprints/OfficeGuy/GDTB_OfficeGuy_Anim_OfficeGuy_Use.GDTB_OfficeGuy_Anim_OfficeGuy_Use" false)
  (`KismetSystemLibrary.Delay` 0.25)
  (`CharacterMovementComponent.SetMovementMode` (`self.CharacterMovement`) "MOVE_Walking" 0)
  (`SkeletalMeshComponent.SetAnimationMode` (`self.Mesh`) "AnimationBlueprint"))

(fn `UserConstructionScript`)