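; BP_RandomAnnouncements periodically shows announcements from "The Boss" on screen.
; On BeginPlay it creates a W_Announcement widget, adds it to the viewport, and starts a looping timer built from Delay nodes.
; After an initial delay, it waits a random interval, then announces either the next entry in RandomAnnouncements, wrapping by modulo, or a random one, depending on IsSequential.
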(event `self.ReceiveBeginPlay`
  (bind _returnvalue (`|CreateWidget` "/Game/MyContent/Blueprints/W_Announcement.W_Announcement_C" (`GameplayStatics.GetPlayerController` 0)))
  (set `self.AnnouncementWidget` _returnvalue)
  (`UserWidget.AddToViewport` (`self.AnnouncementWidget`) 0)
  (`self.Start`))

(event `Start`
  (bind _randomannouncements (`self.RandomAnnouncements`))
  (bind _randomannouncements_2 (`self.RandomAnnouncements`))
  (`KismetSystemLibrary.Delay` (`self.InitialDelay`))
  (`KismetSystemLibrary.Delay` (`KismetMathLibrary.RandomFloatInRange` (`self.RandomDelayMin`) (`self.RandomDelayMax`)) :!label _label)
  (if (`self.bIsSequential`)
    (`/Game/MyContent/Blueprints/W_Announcement.Announce` (`self.AnnouncementWidget`) "The Boss" (`|GetArrayItem` _randomannouncements (mod (`self.Index`) (`KismetArrayLibrary.Array_Length` _randomannouncements))) 8.0)
    (`/Engine/EditorBlueprintResources/StandardMacros.IncrementInt` (`self.Index`)
      (:`  `
        (goto _label)))
    (else
      (`/Game/MyContent/Blueprints/W_Announcement.Announce` (`self.AnnouncementWidget`) "The Boss" (`|GetArrayItem` _randomannouncements_2 (`KismetMathLibrary.RandomIntegerInRange` 0 (- (`KismetArrayLibrary.Array_Length` _randomannouncements_2) 1))) 8.0)
      (goto _label))))

(fn `UserConstructionScript`)